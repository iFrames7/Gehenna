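; Base interactable Blueprint that plays a scene's dialogue, advancing one line per Interact call.
; On BeginPlay it looks up CurrentSceneID in DT_SceneManager to get that scene's DataTable, then steps through its rows by index.
; Each row fills WBP_Dialogue with speaker, text, expression and a portrait chosen by hard-coded name check.
; A DoOnce locks player move and look input until the last line, when the widget and index reset.
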(event Custom|SwitchInput
  (params (isActive :type Boolean))
  (bind _returnvalue (Game|GetPlayerController 0))
  (Input|SetIgnoreMoveInput _returnvalue isActive)
  (Input|SetIgnoreLookInput _returnvalue isActive))

(event EventInteract
  ;[1 1 1] Al interactuar con este objeto...
  (Utilities|FlowControl|Sequence
    (:then_0
      ;[1 1 1] La primera vez, se desabilita el movimiento y la cámara
      (Utilities|FlowControl|DoOnce false :!label _label
        (:Completed
          (CallFunction|SwitchInput true))))
    (:then_1
      ;[1 1 1] Se incrementa el dialogueIndex para saber en qué línea está el diálogo actual
      (bind _result (Math|Integer|IncrementInt (Variables|Default|GetdialogueIndex))
        (:%20%20
          (bind _output_get (Variables|Default|SetdialogueIndex _result))
          (bind _outrownames (DataTable|GetDataTableRowNames (Variables|Default|GetcurrentSceneDataTable)))
          ;[1 1 1] Check para saber si el dialogo se terminó
          (if (< _output_get (Utilities|Array|Length _outrownames))
            ;[1 1 1] Si aún no termina, se settean variables como el texto, nombre del personaje y expresión basado en el dialogueIndex
            (CallFunction|SetVariablesforDialogue _output_get)
            ;[1 1 1] Si no existe el UI, se crea y se settea el texto e imagenes. Si sí existe, se settea el texto y las imagenes
            (Variables|Default|GetdialogueUI
              (:then
                _)
              (:else
                (bind _returnvalue (UserInterface|CreateWidget "/Game/Gehenna/Core/UI/WBP_Dialogue.WBP_Dialogue_C"))
                (bind _output_get_2 (Variables|Default|SetdialogueUI _returnvalue))
                (UserInterface|Viewport|AddtoViewport _output_get_2 0)))
            (CallFunction|SetUITextandImage)
            (else
              ;[1 1 1] Si ya terminó, se quita el UI de la pantalla, se resetea el dialogueIndex y se rehabilitan el movimiento y la camara
              (Widget|RemovefromParent (Variables|Default|GetdialogueUI))
              (Variables|Default|SetdialogueUI 0)
              (Variables|Default|SetdialogueIndex -1)
              (CallFunction|SwitchInput false)
              (goto _label Reset))))))))

(event EventBeginPlay
  ;[1 1 1] Al iniciar, se establece que DT de dialogo se usara basado en la variable currentSceneID
  (CallFunction|SetSceneDataTable))

(fn ConstructionScript)

(fn SetSceneDataTable
  (bind _returnvalue (Utilities|GetDataTableRow "/Game/Gehenna/Dialogues/DT_SceneManager.DT_SceneManager" (Variables|Default|GetcurrentSceneID))
    (:then
      (Variables|Default|SetcurrentSceneDataTable (.scenedt _returnvalue)))))

(fn SetVariablesforDialogue
  (params (dialogueIndex :type Integer))
  (bind _outrownames (DataTable|GetDataTableRowNames (Variables|Default|GetcurrentSceneDataTable)))
  (bind _returnvalue (Utilities|GetDataTableRow (Variables|Default|GetcurrentSceneDataTable) (Utilities|Array|Get(acopy) _outrownames dialogueIndex))
    (:then
      (bind _output_get (Variables|Default|SetsceneDataStruct _returnvalue))
      (bind _output_get_2 (Variables|Default|SetcharacterName (.Speaker (Utilities|Struct|BreakS_SceneDialogueData _output_get))))
      (Variables|Default|SetdialogueText (.Text (Utilities|Struct|BreakS_SceneDialogueData _output_get)))
      (if (== _output_get_2 "Bol Sadguy")
        (Variables|Default|SetcharacterSprite "/Game/Gehenna/Art/PlaceHolders/Bol_Sadguy.Bol_Sadguy")
        (else
          (Variables|Default|SetcharacterSprite "/Engine/EngineResources/AICON-Green.AICON-Green")))
      (Variables|Default|Setexpression (.Expression (Utilities|Struct|BreakS_SceneDialogueData _output_get))))))

(fn SetUITextandImage
  (bind _dialogueui (Variables|Default|GetdialogueUI))
  (Rendering|Components|TextRender|SetText (Variables|/Game/Gehenna/Core/UI/WBP_Dialogue.WBP_Dialogue_C|GetText _dialogueui) (Utilities|Text|ToText(String) (Variables|Default|GetdialogueText)))
  (Rendering|Components|TextRender|SetText (Variables|/Game/Gehenna/Core/UI/WBP_Dialogue.WBP_Dialogue_C|GetCharacterName _dialogueui) (Utilities|Text|ToText(Name) (Variables|Default|GetcharacterName)))
  (Appearance|SetBrushfromTexture (Variables|/Game/Gehenna/Core/UI/WBP_Dialogue.WBP_Dialogue_C|GetCharacterSprite _dialogueui) (Variables|Default|GetcharacterSprite) true)
  (Rendering|Components|TextRender|SetText (Variables|/Game/Gehenna/Core/UI/WBP_Dialogue.WBP_Dialogue_C|GetExpression _dialogueui) (Utilities|Text|ToText(String) (Utilities|String|EnumtoString (Variables|Default|Getexpression)))))

(fn GetInteractName
  (return (Variables|Default|GetinteractName)))

(fn IsInteractable
  (return true))