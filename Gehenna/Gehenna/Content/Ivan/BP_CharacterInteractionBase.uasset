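; Base interactable character that plays a scene's dialogue one line per interaction.
; On BeginPlay it resolves the current scene's dialogue table by looking up the scene ID in DT_SceneReferencer.
; Each Interact reads the next row by index and fills a WBP_Dialogue widget with speaker, text, expression and a sprite picked by a hardcoded name check.
; Past the last row, it removes the widget and resets the index.
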(event EventInteract
  (bind _result (Math|Integer|IncrementInt (Variables|Default|GetdialogueIndex))
    (:%20%20
      (bind _output_get (Variables|Default|SetdialogueIndex _result))
      (bind _outrownames (DataTable|GetDataTableRowNames (Variables|Default|GetcurrentSceneDataTable)))
      (CallFunction|SetVariablesforDialogue _output_get)
      (if (< _output_get (Utilities|Array|Length _outrownames))
        (Variables|Default|GetdialogueUI
          (:then
            _)
          (:else
            (bind _returnvalue (UserInterface|CreateWidget "/Game/Ivan/WBP_Dialogue.WBP_Dialogue_C"))
            (bind _output_get_2 (Variables|Default|SetdialogueUI _returnvalue))
            (UserInterface|Viewport|AddtoViewport _output_get_2 0)))
        (CallFunction|SetUITextandImage)
        (else
          (Widget|RemovefromParent (Variables|Default|GetdialogueUI))
          (Variables|Default|SetdialogueUI 0)
          (Variables|Default|SetdialogueIndex -1))))))

(event EventBeginPlay
  (CallFunction|SetSceneDataTable))

(fn ConstructionScript)

(fn SetSceneDataTable
  (bind _returnvalue (Utilities|GetDataTableRow "/Game/Ivan/DT_SceneReferencer.DT_SceneReferencer" (Variables|Default|GetcurrentSceneID))
    (:then
      (Variables|Default|SetcurrentSceneDataTable (.scenedt _returnvalue)))))

(fn SetVariablesforDialogue
  (params (dialogueIndex :type Integer))
  (bind _outrownames (DataTable|GetDataTableRowNames (Variables|Default|GetcurrentSceneDataTable)))
  (bind _returnvalue (Utilities|GetDataTableRow (Variables|Default|GetcurrentSceneDataTable) (Utilities|Array|Get(acopy) _outrownames dialogueIndex))
    (:then
      (bind _output_get (Variables|Default|SetsceneDataStruct _returnvalue))
      (bind _output_get_2 (Variables|Default|SetcharacterName (.Speaker (Utilities|Struct|BreakS_SceneDialogueData _output_get))))
      (Variables|Default|SetdialogueText (.Text (Utilities|Struct|BreakS_SceneDialogueData _output_get)))
      (if (== _output_get_2 "Bol Sadguy")
        (Variables|Default|SetcharacterSprite "/Game/Ivan/Bol_Sadguy.Bol_Sadguy")
        (else
          (Variables|Default|SetcharacterSprite "/Engine/EngineResources/AICON-Green.AICON-Green")))
      (Variables|Default|Setexpression (.Expression (Utilities|Struct|BreakS_SceneDialogueData _output_get))))))

(fn SetUITextandImage
  (bind _dialogueui (Variables|Default|GetdialogueUI))
  (Rendering|Components|TextRender|SetText (Variables|/Game/Ivan/WBP_Dialogue.WBP_Dialogue_C|GetText _dialogueui) (Utilities|Text|ToText(String) (Variables|Default|GetdialogueText)))
  (Rendering|Components|TextRender|SetText (Variables|/Game/Ivan/WBP_Dialogue.WBP_Dialogue_C|GetCharacterName _dialogueui) (Utilities|Text|ToText(Name) (Variables|Default|GetcharacterName)))
  (Appearance|SetBrushfromTexture (Variables|/Game/Ivan/WBP_Dialogue.WBP_Dialogue_C|GetCharacterSprite _dialogueui) (Variables|Default|GetcharacterSprite) true)
  (Rendering|Components|TextRender|SetText (Variables|/Game/Ivan/WBP_Dialogue.WBP_Dialogue_C|GetExpression _dialogueui) (Utilities|Text|ToText(String) (Utilities|String|EnumtoString (Variables|Default|Getexpression)))))

(fn GetInteractName
  (return (Variables|Default|GetinteractName)))

(fn IsInteractable
  (return true))